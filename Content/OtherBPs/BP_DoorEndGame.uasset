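; End-of-game door actor that wins the game when the paper cat character reaches it with every fish collected.
; On BeginPlay it counts all BP_Fish actors in the level to set the required total.
; When the player overlaps its box and their fish count equals that total, it shows the HUD's win screen, pauses the game and switches to cursor-driven, UI-only input.
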(event `self.ReceiveBeginPlay`
  (bind _outactors (`GameplayStatics.GetAllActorsOfClass` "/Game/OtherBPs/BP_Fish.BP_Fish_C"))
  (set `self.Fishrequired` (`KismetArrayLibrary.Array_Length` _outactors)))

(event `self.Box.OnComponentBeginOverlap`
  (params (OverlappedComponent :type "PrimitiveComponent Object Reference") (OtherActor :type "Actor Object Reference") (OtherComp :type "PrimitiveComponent Object Reference") (OtherBodyIndex :type Integer) (bFromSweep :type Boolean) (SweepResult :type "HitResult Structure (by ref)"))
  (bind _returnvalue (`GameplayStatics.GetPlayerController` 0))
  (bind _asbp_paper_cat_characte (cast `/Game/PaperCatCharacter/BP_PaperCatCharacte` OtherActor))
  (if (== (`/Game/PaperCatCharacter/BP_PaperCatCharacte.Fish` _asbp_paper_cat_characte) (`self.Fishrequired`))
    (`Widget.SetVisibility` (`/Game/UI/WB_Timer.GameWonScreen` (`/Game/PaperCatCharacter/BP_PaperCatCharacte.PlayerHUD ref` _asbp_paper_cat_characte)) "Visible")
    (`GameplayStatics.SetGamePaused` true)
    (set `PlayerController.bShowMouseCursor` true _returnvalue)
    (`WidgetBlueprintLibrary.SetInputMode_UIOnlyEx` _returnvalue null)))

(fn `UserConstructionScript`)