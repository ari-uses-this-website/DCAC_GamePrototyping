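; BP_PaperCatCharacte is the player's side-scrolling 2D cat character, with movement, health and a level countdown.
; Enhanced Input drives movement along X with sprite flipping, plus jumping and a Jump flag on the animation Blueprint.
; Tick updates the timer HUD; TakeDamage updates health and plays a Scare override.
; Time running out or health equalling zero shows Game Over and pauses with UI-only input; HealthPickUp is an empty stub.
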(event `self.ReceiveTick`
  (params (DeltaSeconds :type "Float (single-precision)"))
  (bind _output_get (set `self.Time Amount` (`KismetMathLibrary.FClamp` (- (`self.Time Amount`) (`GameplayStatics.GetWorldDeltaSeconds`)) 0.0 (`self.Time Amount`))))
  (if (> _output_get 0.0)
    (`TextBlock.SetText` (`/Game/UI/WB_Timer.TimeCountdown` (`self.PlayerHUD ref`)) (`KismetTextLibrary.Conv_StringToText` (`KismetStringLibrary.TimeSecondsToString` _output_get)))
    (else
      (`Widget.SetVisibility` (`/Game/UI/WB_Timer.GameOverScreen` (`self.PlayerHUD ref`)) "Visible")
      (`self.Death Operation`))))

(event `self.ReceiveBeginPlay`
  (`|ExecutionSequence`
    (:`then_0`
      (`EnhancedInputSubsystemInterface.AddMappingContext` (pcsubsystem `EnhancedInputLocalPlayerSubsystem` (`GameplayStatics.GetPlayerController` 0)) "/Game/PaperCatCharacter/IAM_PaperCatCharacter.IAM_PaperCatCharacter" 0 (struct))
      (bind _asabp_character (cast `/Game/PaperCatCharacter/ABP_Character` (`PaperZDAnimationComponent.AnimInstance` (`self.AnimationComponent`))))
      (set `self.As ABP Character` _asabp_character))
    (:`then_1`
      (bind _returnvalue (`|CreateWidget` "/Game/UI/WB_Timer.WB_Timer_C"))
      (bind _output_get (set `self.PlayerHUD ref` _returnvalue))
      (`UserWidget.AddToViewport` _returnvalue 0)
      (`UserWidget.AddToViewport` _output_get 0))))

(event `EnhancedInput|/Game/PaperCatCharacter/PaperCatCharacterIA/IA_Move`
  (params (ActionValue :type "Float (double-precision)") (ElapsedSeconds :type "Float (double-precision)") (TriggeredSeconds :type "Float (double-precision)") (InputAction :type "InputAction Object Reference" :default "/Game/PaperCatCharacter/PaperCatCharacterIA/IA_Move.IA_Move"))
  (:`Triggered`
    (`self.AddMovementInput` (1.0 0.0 0.0) ActionValue)
    (`SceneComponent.K2_SetRelativeRotation` (`self.Sprite`) (select `bool` (> ActionValue 0.0) :`true` (struct :`Yaw` -180.0) :!type "Rotator Structure") false false)))

(event `EnhancedInput|/Game/PaperCatCharacter/PaperCatCharacterIA/IA_Jump`
  (params (ActionValue :type Boolean) (ElapsedSeconds :type "Float (double-precision)") (TriggeredSeconds :type "Float (double-precision)") (InputAction :type "InputAction Object Reference" :default "/Game/PaperCatCharacter/PaperCatCharacterIA/IA_Jump.IA_Jump"))
  (:`Started`
    (`self.Jump`)
    (set `/Game/PaperCatCharacter/ABP_Character.Jump` true (`self.As ABP Character`)))
  (:`Completed`
    (`self.StopJumping`)))

(event `self.OnLanded`
  (params (Hit :type "HitResult Structure (by ref)"))
  (set `/Game/PaperCatCharacter/ABP_Character.Jump` false (`self.As ABP Character`)))

(fn `Death Operation`
  (bind _returnvalue (`GameplayStatics.GetPlayerController` 0))
  (`GameplayStatics.SetGamePaused` true)
  (set `PlayerController.bShowMouseCursor` true _returnvalue)
  (`WidgetBlueprintLibrary.SetInputMode_UIOnlyEx` _returnvalue null))

(fn `HealthPickUp`)

(fn `Take Damage`
  (params (Damage :type Integer))
  (bind _output_get (set `self.Health` (- (`self.Health`) Damage)))
  (`/Game/UI/WB_Timer.UpdateHealth` (`self.PlayerHUD ref`) _output_get)
  (`PaperZDAnimInstance.K2_PlayAnimationOverride` (`self.As ABP Character`) "/Game/PaperCatCharacter/CatSprites/AnimSequences/Scare.Scare" "DefaultSlot" 1.0 0.0)
  (if (== _output_get 0)
    (`Widget.SetVisibility` (`/Game/UI/WB_Timer.GameOverScreen` (`self.PlayerHUD ref`)) "Visible")
    (`self.Death Operation`)))

(fn `UserConstructionScript`)