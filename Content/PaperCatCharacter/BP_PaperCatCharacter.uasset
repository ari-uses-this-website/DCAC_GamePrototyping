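; Player-controlled 2D paper cat character that runs a countdown timer and tracks health, ending the game when either runs out.
; Enhanced Input drives single-axis movement with sprite flipping and jumping, which sets a flag on the animation blueprint and plays sounds.
; A timer widget created at BeginPlay shows time and health.
; TakeDamage plays a scare animation override; game over pauses play and switches to UI-only input.
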(event `CustomEvent`)

(event `self.ReceiveTick`
  (params (DeltaSeconds :type "Float (single-precision)"))
  (bind _returnvalue (`GameplayStatics.GetPlayerController` 0))
  (bind _output_get (set `self.TimeValue` (`KismetMathLibrary.FClamp` (- (`self.TimeValue`) (`GameplayStatics.GetWorldDeltaSeconds`)) 0.0 (`self.TimeValue`))))
  (if (> _output_get 0.0)
    (`TextBlock.SetText` (`/Game/UI/WB_Timer.TimeCountdown` (`self.Player HUD`)) (`KismetTextLibrary.Conv_StringToText` (`KismetStringLibrary.TimeSecondsToString` _output_get)))
    (else
      (`Widget.SetVisibility` (`/Game/UI/WB_Timer.GameOverScreen` (`self.Player HUD`)) "Visible")
      (`GameplayStatics.SetGamePaused` true)
      (set `PlayerController.bShowMouseCursor` true _returnvalue)
      (`WidgetBlueprintLibrary.SetInputMode_UIOnlyEx` _returnvalue null))))

(event `self.ReceiveBeginPlay`
  (`|ExecutionSequence`
    (:`then_0`
      (`EnhancedInputSubsystemInterface.AddMappingContext` (pcsubsystem `EnhancedInputLocalPlayerSubsystem` (`GameplayStatics.GetPlayerController` 0)) "/Game/PaperCatCharacter/IAM_PaperCatCharacter.IAM_PaperCatCharacter" 0 (struct))
      (bind _asabp_paper_cha_cat (cast `/Game/PaperCatCharacter/CatSprites/ABP_PaperChaCat` (`PaperZDAnimationComponent.AnimInstance` (`self.AnimationComponent`))))
      (set `self.As ABP Paper Cha Cat` _asabp_paper_cha_cat))
    (:`then_1`
      (bind _returnvalue (`|CreateWidget` "/Game/UI/WB_Timer.WB_Timer_C"))
      (bind _output_get (set `self.Player HUD` _returnvalue))
      (`UserWidget.AddToViewport` _output_get 0)
      (`UserWidget.AddToViewport` _returnvalue 0)
      (`/Game/UI/WB_Timer.UpdateHealth` _returnvalue (`self.PlayerHealth`)))))

(event `EnhancedInput|/Game/PaperCatCharacter/PaperCatCharacterIA/IA_Run`
  (params (ActionValue :type "Float (double-precision)") (ElapsedSeconds :type "Float (double-precision)") (TriggeredSeconds :type "Float (double-precision)") (InputAction :type "InputAction Object Reference" :default "/Game/PaperCatCharacter/PaperCatCharacterIA/IA_Run.IA_Run")))

(event `EnhancedInput|/Game/PaperCatCharacter/PaperCatCharacterIA/IA_Move`
  (params (ActionValue :type "Float (double-precision)") (ElapsedSeconds :type "Float (double-precision)") (TriggeredSeconds :type "Float (double-precision)") (InputAction :type "InputAction Object Reference" :default "/Game/PaperCatCharacter/PaperCatCharacterIA/IA_Move.IA_Move"))
  (:`Triggered`
    (`self.AddMovementInput` (1.0 0.0 0.0) ActionValue)
    (`SceneComponent.K2_SetRelativeRotation` (`self.Sprite`) (select `bool` (> ActionValue 0.0) :`true` (struct :`Yaw` -180.0) :!type "Rotator Structure") false false)))

(event `EnhancedInput|/Game/PaperCatCharacter/PaperCatCharacterIA/IA_Jump`
  (params (ActionValue :type Boolean) (ElapsedSeconds :type "Float (double-precision)") (TriggeredSeconds :type "Float (double-precision)") (InputAction :type "InputAction Object Reference" :default "/Game/PaperCatCharacter/PaperCatCharacterIA/IA_Jump.IA_Jump"))
  (:`Started`
    (`self.Jump`)
    (set `/Game/PaperCatCharacter/CatSprites/ABP_PaperChaCat.Jumping` true (`self.As ABP Paper Cha Cat`))
    (`GameplayStatics.PlaySound2D` "/Game/Sounds/Jump.Jump" 1.0 1.0 0.0 null null))
  (:`Completed`
    (`self.StopJumping`)))

(event `self.OnLanded`
  (params (Hit :type "HitResult Structure (by ref)"))
  (set `/Game/PaperCatCharacter/CatSprites/ABP_PaperChaCat.Jumping` false (`self.As ABP Paper Cha Cat`))
  (`GameplayStatics.PlaySound2D` "/Game/Sounds/SoftThud.SoftThud" 1.0 1.0 0.0 null null))

(event `self.ScareBox.OnComponentBeginOverlap`
  (params (OverlappedComponent :type "PrimitiveComponent Object Reference") (OtherActor :type "Actor Object Reference") (OtherComp :type "PrimitiveComponent Object Reference") (OtherBodyIndex :type Integer) (bFromSweep :type Boolean) (SweepResult :type "HitResult Structure (by ref)")))

(fn `TakeDamage`
  (params (Damage :type Integer))
  (bind _returnvalue (`GameplayStatics.GetPlayerController` 0))
  (bind _output_get (set `self.PlayerHealth` (- (`self.PlayerHealth`) Damage)))
  (`/Game/UI/WB_Timer.UpdateHealth` (`self.Player HUD`) (`self.PlayerHealth`))
  (`PaperZDAnimInstance.K2_PlayAnimationOverride` (`self.As ABP Paper Cha Cat`) "/Game/PaperCatCharacter/CatSprites/AnimSequences/Scare.Scare" "DefaultSlot" 1.0 0.0)
  (if (== _output_get 0)
    (`KismetSystemLibrary.PrintString` "NO MONEY")
    (`Widget.SetVisibility` (`/Game/UI/WB_Timer.GameOverScreen` (`self.Player HUD`)) "Visible")
    (`WidgetBlueprintLibrary.SetInputMode_UIOnlyEx` _returnvalue null)
    (set `PlayerController.bShowMouseCursor` true _returnvalue)
    (`GameplayStatics.SetGamePaused` true)
    (else
      (`KismetSystemLibrary.PrintString` (`KismetStringLibrary.Conv_IntToString` _output_get)))))

(fn `UserConstructionScript`)